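; GeneralSam_BP is a player character with third-person movement and physically animated body motion.
; On possession it adds the third-person Enhanced Input mapping context; move inputs follow control yaw, and look input drives scaled yaw only.
; On BeginPlay, PhysicalAnimationSam applies the "Body" profile to the mesh and enables physics simulation below a configured bone, blending animation with physics.
; An alternative hard-coded physical animation setup is left unconnected.
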(event Input|EnhancedActionEvents|EnhancedInputActionIA_MoveForward_CC
  (params (ActionValue :type Float%20%28double-precision%29) (ElapsedSeconds :type Float%20%28double-precision%29) (TriggeredSeconds :type Float%20%28double-precision%29) (InputAction :type Input%20Action%20Object%20Reference :default "/Game/Game/Inputs/IA_MoveForward_CC.IA_MoveForward_CC"))
  (:Triggered
    (Pawn|Input|AddMovementInput (Math|Vector|GetForwardVector (Math|Rotator|MakeRotator 0.0 0.0 (.Yaw (Math|Rotator|BreakRotator (Pawn|GetControlRotation :!class /Script/Engine.Pawn))))) ActionValue false)))

(event Input|EnhancedActionEvents|EnhancedInputActionIA_MoveRight_CC
  (params (ActionValue :type Float%20%28double-precision%29) (ElapsedSeconds :type Float%20%28double-precision%29) (TriggeredSeconds :type Float%20%28double-precision%29) (InputAction :type Input%20Action%20Object%20Reference :default "/Game/Game/Inputs/IA_MoveRight_CC.IA_MoveRight_CC"))
  (:Triggered
    (Pawn|Input|AddMovementInput (Math|Vector|GetRightVector (Math|Rotator|MakeRotator 0.0 0.0 (.Yaw (Math|Rotator|BreakRotator (Pawn|GetControlRotation :!class /Script/Engine.Pawn))))) ActionValue false)))

(event Input|EnhancedActionEvents|EnhancedInputActionIA_LookAt
  (params (ActionValue :type Float%20%28double-precision%29) (ElapsedSeconds :type Float%20%28double-precision%29) (TriggeredSeconds :type Float%20%28double-precision%29) (InputAction :type Input%20Action%20Object%20Reference :default "/Game/Game/Inputs/IA_LookAt.IA_LookAt"))
  (:Triggered
    (Pawn|Input|AddControllerYawInput (/ ActionValue 3.0))))

(event Input|EnhancedActionEvents|EnhancedInputActionIA_LookAt_Y
  (params (ActionValue :type Float%20%28double-precision%29) (ElapsedSeconds :type Float%20%28double-precision%29) (TriggeredSeconds :type Float%20%28double-precision%29) (InputAction :type Input%20Action%20Object%20Reference :default "/Game/Game/Inputs/IA_LookAt_Y.IA_LookAt_Y")))

(event EventBeginPlay
  (bind _bone (Variables|Default|GetBone))
  (Class|PhysicalAnimationComponent|SetSkeletalMeshComponent (Variables|Default|GetPhysicalAnimation_Sam) (Variables|Character|GetMesh))
  (Class|PhysicalAnimationComponent|ApplyPhysicalAnimationProfileBelow (Variables|Default|GetPhysicalAnimation_Sam) _bone "Body" true false)
  (Class|SkeletalMeshComponent|SetAllBodiesBelowSimulatePhysics (Variables|Character|GetMesh) _bone true false))

(event EventPossessed
  (params (NewController :type Controller%20Object%20Reference))
  (bind _asplayer_controller (Utilities|Casting|CastToPlayerController NewController))
  (Input|AddMappingContext (PlayerController|LocalPlayerSubsystems|GetEnhancedInputLocalPlayerSubsystem _asplayer_controller) "/Game/Game/Inputs/Player_MappingContext_3P.Player_MappingContext_3P" 0 "(bIgnoreAllPressedKeysUntilRelease=True,bForceImmediately=False)"))

(fn ConstructionScript)