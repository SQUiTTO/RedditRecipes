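; Player character with Enhanced Input movement, look and per-finger hand controls for grabbing physics objects.
; Finger inputs set curl values from hold time, alongside look values and state flags.
; Thumb input while the index is held sphere-traces from ThumbCollision along camera forward, grabbing hits with a PhysicsHandle until thumb release.
; UpdateLoc re-calls itself every 0.1 seconds to retarget the handle; physical animation setup is disconnected.
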(event Custom|UpdateLoc
  (bind _thumb_collision (Variables|Default|GetThumb_Collision))
  (Utilities|IsValid (Variables|Default|GetHit%20Component)
    (:Is%20Valid
      (Class|PhysicsHandleComponent|SetTargetLocationandRotation (Variables|Default|GetPhysicsHandle) (Math|Transform|TransformLocation (Transformation|GetWorldTransform _thumb_collision) (Variables|Default|GetImpact%20Point)) (Transformation|GetWorldRotation _thumb_collision))
      (Utilities|FlowControl|Delay 0.1)
      (CallFunction|UpdateLoc))))

(event Input|EnhancedActionEvents|EnhancedInputActionIA_MoveForward_CC
  (params (ActionValue :type Float%20%28double-precision%29) (ElapsedSeconds :type Float%20%28double-precision%29) (TriggeredSeconds :type Float%20%28double-precision%29) (InputAction :type Input%20Action%20Object%20Reference :default "/Game/Game/Inputs/IA_MoveForward_CC.IA_MoveForward_CC"))
  ;[1 1 1] Movement
  (:Triggered
    (Pawn|Input|AddMovementInput (Math|Vector|GetForwardVector (Math|Rotator|MakeRotator 0.0 0.0 (.Yaw (Math|Rotator|BreakRotator (Pawn|GetControlRotation :!class /Script/Engine.Pawn))))) ActionValue false)))

(event Input|EnhancedActionEvents|EnhancedInputActionIA_MoveRight_CC
  (params (ActionValue :type Float%20%28double-precision%29) (ElapsedSeconds :type Float%20%28double-precision%29) (TriggeredSeconds :type Float%20%28double-precision%29) (InputAction :type Input%20Action%20Object%20Reference :default "/Game/Game/Inputs/IA_MoveRight_CC.IA_MoveRight_CC"))
  ;[1 1 1] Movement
  (:Triggered
    (Pawn|Input|AddMovementInput (Math|Vector|GetRightVector (Math|Rotator|MakeRotator 0.0 0.0 (.Yaw (Math|Rotator|BreakRotator (Pawn|GetControlRotation :!class /Script/Engine.Pawn))))) ActionValue false)))

(event Input|EnhancedActionEvents|EnhancedInputActionIA_LookAt
  (params (ActionValue :type Float%20%28double-precision%29) (ElapsedSeconds :type Float%20%28double-precision%29) (TriggeredSeconds :type Float%20%28double-precision%29) (InputAction :type Input%20Action%20Object%20Reference :default "/Game/Game/Inputs/IA_LookAt.IA_LookAt"))
  ;[1 1 1] look at
  (:Triggered
    (Pawn|Input|AddControllerYawInput (/ ActionValue 3.0))
    (Variables|Default|SetLook%20Side ActionValue :!label _label))
  (:Started
    (Variables|Default|SetLooking%20X true)
    (goto _label))
  (:Ongoing
    (Variables|Default|SetLooking%20X false :!label _label_2))
  (:Canceled
    (goto _label_2))
  (:Completed
    (goto _label_2)))

(event Input|EnhancedActionEvents|EnhancedInputActionIA_LookAt_Y
  (params (ActionValue :type Float%20%28double-precision%29) (ElapsedSeconds :type Float%20%28double-precision%29) (TriggeredSeconds :type Float%20%28double-precision%29) (InputAction :type Input%20Action%20Object%20Reference :default "/Game/Game/Inputs/IA_LookAt_Y.IA_LookAt_Y"))
  ;[1 1 1] look at
  (:Triggered
    (Pawn|Input|AddControllerPitchInput ActionValue)
    (Variables|Default|SetLook%20Up (Math|Float|Clamp(Float) (+ (* ActionValue 3e+01) (Variables|Default|GetLook%20Up)) -1e+01 1e+01)))
  (:Started
    (Variables|Default|SetLooking%20Y true))
  (:Canceled
    (Variables|Default|SetLooking%20Y false :!label _label))
  (:Completed
    (goto _label)))

(event Input|EnhancedActionEvents|EnhancedInputActionIA_Index_CC
  (params (ActionValue :type Boolean) (ElapsedSeconds :type Float%20%28double-precision%29) (TriggeredSeconds :type Float%20%28double-precision%29) (InputAction :type Input%20Action%20Object%20Reference :default "/Game/Game/Inputs/IA_Index_CC.IA_Index_CC"))
  ;[1 1 1] Fingers
  (:Triggered
    (Variables|Default|SetIndex (* ElapsedSeconds 1e+01)))
  (:Started
    (Variables|Default|SetRotatedIndex true))
  (:Completed
    (Variables|Default|SetRotatedIndex false)))

(event Input|EnhancedActionEvents|EnhancedInputActionIA_Thumb_CC
  (params (ActionValue :type Boolean) (ElapsedSeconds :type Float%20%28double-precision%29) (TriggeredSeconds :type Float%20%28double-precision%29) (InputAction :type Input%20Action%20Object%20Reference :default "/Game/Game/Inputs/IA_Thumb_CC.IA_Thumb_CC"))
  (bind _camera (Variables|Default|GetCamera))
  (bind _thumb_collision (Variables|Default|GetThumb_Collision))
  (bind _returnvalue (Transformation|GetWorldLocation _thumb_collision))
  (bind _returnvalue_2 (Transformation|GetWorldTransform _camera))
  (:Triggered
    (Variables|Default|SetThumb (* ElapsedSeconds 1e+01))
    (Variables|Default|SetRotatedThumb true)
    (if (Variables|Default|GetRotatedIndex)
      (bind (_outhit _returnvalue_3) (Collision|SphereTraceByChannel _returnvalue (+ _returnvalue (* (Math|Vector|GetForwardVector (Transformation|GetWorldRotation (Variables|Default|GetCamera))) 15.0)) 7.0 "TraceTypeQuery1" true 0 "ForDuration"))
      (if _returnvalue_3
        (bind _output_get (Variables|Default|SetImpact%20Point (.ImpactPoint (Collision|BreakHitResult _outhit))))
        (bind _output_get_2 (Variables|Default|SetHit%20Component (.HitComponent (Collision|BreakHitResult _outhit))))
        (Physics|Components|PhysicsHandle|GrabComponentatLocationwithRotation (Variables|Default|GetPhysicsHandle) _output_get_2 "None" _output_get (Math|Transform|InverseTransformRotation _returnvalue_2 (Transformation|GetWorldRotation _camera)))
        (Variables|Default|SetCanHold true)
        (Variables|Default|SetImpact%20Point (Math|Transform|InverseTransformLocation _returnvalue_2 (Variables|Default|GetImpact%20Point)))
        (CallFunction|UpdateLoc))))
  (:Completed
    (Variables|Default|SetRotatedThumb false)
    (if (Variables|Default|GetCanHold)
      (Physics|Components|PhysicsHandle|ReleaseComponent (Variables|Default|GetPhysicsHandle))
      (Variables|Default|SetCanHold false))))

(event Input|EnhancedActionEvents|EnhancedInputActionIA_OtherFingers_CC
  (params (ActionValue :type Boolean) (ElapsedSeconds :type Float%20%28double-precision%29) (TriggeredSeconds :type Float%20%28double-precision%29) (InputAction :type Input%20Action%20Object%20Reference :default "/Game/Game/Inputs/IA_OtherFingers_CC.IA_OtherFingers_CC"))
  ;[1 1 1] Fingers
  (:Triggered
    (Variables|Default|SetOtherFingers (* ElapsedSeconds 8e+01))
    (Variables|Default|SetRotatedOtherFings true))
  (:Completed
    (Variables|Default|SetRotatedOtherFings false)))

(event EventBeginPlay
  ;[1 1 1] Fizicks
)

(event EventPossessed
  (params (NewController :type Controller%20Object%20Reference))
  (bind _asplayer_controller (Utilities|Casting|CastToPlayerController NewController))
  (Input|AddMappingContext (PlayerController|LocalPlayerSubsystems|GetEnhancedInputLocalPlayerSubsystem _asplayer_controller) "/Game/Game/Inputs/Player_MappingContext_3P.Player_MappingContext_3P" 0 "(bIgnoreAllPressedKeysUntilRelease=True,bForceImmediately=False)"))

(fn ConstructionScript)