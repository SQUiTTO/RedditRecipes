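; Component for GeneralSam_BP that adds physics-driven animation to the character's upper body from spine_01 down the bone chain.
; On BeginPlay it creates a PhysicalAnimationComponent on the owner and binds it to the character's mesh.
; TogglePhysicalAnimation simulates spine_01 and the bodies below it, then applies the "Body" profile at full strength.
; Despite its name, the toggle event only switches the effect on.
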(event Custom|TogglePhysicalAnimation
  (bind _physicalanimationcomponent (Variables|Default|GetPhysicalAnimationComponent))
  (Class|SkeletalMeshComponent|SetAllBodiesBelowSimulatePhysics (Variables|Default|GetMesh) (Utilities|Name|MakeLiteralName "spine_01") true true)
  (Class|PhysicalAnimationComponent|ApplyPhysicalAnimationProfileBelow _physicalanimationcomponent "spine_01" "Body" true false)
  (Class|PhysicalAnimationComponent|SetStrengthMultiplyer _physicalanimationcomponent 1.0))

(event EventBeginPlay
  (bind _returnvalue (Game|AddComponentbyClass (Components|GetOwner) "/Script/Engine.PhysicalAnimationComponent"))
  (bind _output_get (Variables|Default|SetPhysicalAnimationComponent _returnvalue))
  (bind _asgeneral_sam_bp (Utilities|Casting|CastToGeneralSam_BP (Components|GetOwner)))
  (Class|PhysicalAnimationComponent|SetSkeletalMeshComponent _output_get (Variables|/Script/Engine.Character|GetMesh _asgeneral_sam_bp))
  (Variables|Default|SetMesh (Variables|/Script/Engine.Character|GetMesh _asgeneral_sam_bp)))