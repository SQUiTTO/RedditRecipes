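; Player character with a physically animated ragdoll hand whose fingers and arm are driven individually through Enhanced Input.
; Finger hold times set rotation values; look input also feeds sway variables.
; Thumb plus an overlapping index or middle finger, or the other fingers, sphere-traces and grabs with a PhysicsHandle, updated camera-relative by a delayed recursive event until invalid.
; Arm extend and raise modes slow walking and lock look input.
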(event OnComponentBeginOverlap(Thumb_Collision)
  (params (OverlappedComponent :type Primitive%20Component%20Object%20Reference) (OtherActor :type Actor%20Object%20Reference) (OtherComp :type Primitive%20Component%20Object%20Reference) (OtherBodyIndex :type Integer) (bFromSweep :type Boolean) (SweepResult :type Hit%20Result%20Structure%20%28by%20ref%29)))

(event OnComponentEndOverlap(Thumb_Collision)
  (params (OverlappedComponent :type Primitive%20Component%20Object%20Reference) (OtherActor :type Actor%20Object%20Reference) (OtherComp :type Primitive%20Component%20Object%20Reference) (OtherBodyIndex :type Integer)))

(event OnComponentBeginOverlap(Ring_Collision)
  (params (OverlappedComponent :type Primitive%20Component%20Object%20Reference) (OtherActor :type Actor%20Object%20Reference) (OtherComp :type Primitive%20Component%20Object%20Reference) (OtherBodyIndex :type Integer) (bFromSweep :type Boolean) (SweepResult :type Hit%20Result%20Structure%20%28by%20ref%29))
  (Variables|Default|SetRingOverlapped true))

(event OnComponentBeginOverlap(Index_Collision)
  (params (OverlappedComponent :type Primitive%20Component%20Object%20Reference) (OtherActor :type Actor%20Object%20Reference) (OtherComp :type Primitive%20Component%20Object%20Reference) (OtherBodyIndex :type Integer) (bFromSweep :type Boolean) (SweepResult :type Hit%20Result%20Structure%20%28by%20ref%29))
  (Variables|Default|SetIndexOverlapped true))

(event OnComponentEndOverlap(Index_Collision)
  (params (OverlappedComponent :type Primitive%20Component%20Object%20Reference) (OtherActor :type Actor%20Object%20Reference) (OtherComp :type Primitive%20Component%20Object%20Reference) (OtherBodyIndex :type Integer))
  (Variables|Default|SetIndexOverlapped false))

(event OnComponentBeginOverlap(Mid_Collision)
  (params (OverlappedComponent :type Primitive%20Component%20Object%20Reference) (OtherActor :type Actor%20Object%20Reference) (OtherComp :type Primitive%20Component%20Object%20Reference) (OtherBodyIndex :type Integer) (bFromSweep :type Boolean) (SweepResult :type Hit%20Result%20Structure%20%28by%20ref%29))
  (Variables|Default|SetMiddle%20Overlapped true))

(event OnComponentEndOverlap(Mid_Collision)
  (params (OverlappedComponent :type Primitive%20Component%20Object%20Reference) (OtherActor :type Actor%20Object%20Reference) (OtherComp :type Primitive%20Component%20Object%20Reference) (OtherBodyIndex :type Integer))
  (Variables|Default|SetMiddle%20Overlapped false))

(event OnComponentEndOverlap(Ring_Collision)
  (params (OverlappedComponent :type Primitive%20Component%20Object%20Reference) (OtherActor :type Actor%20Object%20Reference) (OtherComp :type Primitive%20Component%20Object%20Reference) (OtherBodyIndex :type Integer))
  (Variables|Default|SetRingOverlapped false))

(event Custom|UpdateLoc
  (bind _camera (Variables|Default|GetCamera))
  ;[1 1 1] Comment
  (Utilities|IsValid (Variables|Default|GetHit%20Component)
    (:Is%20Valid
      (Class|PhysicsHandleComponent|SetTargetLocationandRotation (Variables|Default|GetPhysicsHandle) (Math|Transform|TransformLocation (Transformation|GetWorldTransform _camera) (Variables|Default|GetImpact%20Point)) (Transformation|GetWorldRotation _camera))
      (Utilities|FlowControl|Delay 0.01)
      (CallFunction|UpdateLoc))))

(event Input|EnhancedActionEvents|EnhancedInputActionIA_MoveForward_CC
  (params (ActionValue :type Float%20%28double-precision%29) (ElapsedSeconds :type Float%20%28double-precision%29) (TriggeredSeconds :type Float%20%28double-precision%29) (InputAction :type Input%20Action%20Object%20Reference :default "/Game/Game/Inputs/IA_MoveForward_CC.IA_MoveForward_CC"))
  ;[1 1 1] MOVEMENT
  (:Triggered
    (Pawn|Input|AddMovementInput (Math|Vector|GetForwardVector (Math|Rotator|MakeRotator 0.0 0.0 (.Yaw (Math|Rotator|BreakRotator (Pawn|GetControlRotation :!class /Script/Engine.Pawn))))) ActionValue false)))

(event Input|EnhancedActionEvents|EnhancedInputActionIA_MoveRight_CC
  (params (ActionValue :type Float%20%28double-precision%29) (ElapsedSeconds :type Float%20%28double-precision%29) (TriggeredSeconds :type Float%20%28double-precision%29) (InputAction :type Input%20Action%20Object%20Reference :default "/Game/Game/Inputs/IA_MoveRight_CC.IA_MoveRight_CC"))
  ;[1 1 1] MOVEMENT
  (:Triggered
    (Pawn|Input|AddMovementInput (Math|Vector|GetRightVector (Math|Rotator|MakeRotator 0.0 0.0 (.Yaw (Math|Rotator|BreakRotator (Pawn|GetControlRotation :!class /Script/Engine.Pawn))))) ActionValue false)))

(event Input|EnhancedActionEvents|EnhancedInputActionIA_LookAt_Y
  (params (ActionValue :type Float%20%28double-precision%29) (ElapsedSeconds :type Float%20%28double-precision%29) (TriggeredSeconds :type Float%20%28double-precision%29) (InputAction :type Input%20Action%20Object%20Reference :default "/Game/Game/Inputs/IA_LookAt_Y.IA_LookAt_Y"))
  ;[1 1 1] LOOK AT
  (:Triggered
    (Pawn|Input|AddControllerPitchInput ActionValue)
    (Variables|Default|SetLooking%20Y true :!label _label)
    (Utilities|FlowControl|Delay 0.05)
    (if (Variables|Default|GetLooking%20Y)
      (Variables|Default|SetUpLook (* ActionValue 14.0))
      (Variables|Default|SetLooking%20Y false :!label _label_2)))
  (:Started
    (goto _label))
  (:Ongoing
    (goto _label_2))
  (:Canceled
    (goto _label_2))
  (:Completed
    (goto _label_2)))

(event Input|EnhancedActionEvents|EnhancedInputActionIA_LookAt
  (params (ActionValue :type Float%20%28double-precision%29) (ElapsedSeconds :type Float%20%28double-precision%29) (TriggeredSeconds :type Float%20%28double-precision%29) (InputAction :type Input%20Action%20Object%20Reference :default "/Game/Game/Inputs/IA_LookAt.IA_LookAt"))
  ;[1 1 1] LOOK AT
  (:Triggered
    (Pawn|Input|AddControllerYawInput ActionValue))
  (:Started
    (Variables|Default|SetLookingX true)
    (if (Variables|Default|GetLookingX)
      (Utilities|FlowControl|Delay 0.1))
    (Variables|Default|SetSideLook (* ActionValue 7.0)))
  (:Canceled
    (Variables|Default|SetLookingX false :!label _label)
    (Utilities|FlowControl|Delay 0.1))
  (:Completed
    (goto _label)))

(event Input|EnhancedActionEvents|EnhancedInputActionIA_Index_CC
  (params (ActionValue :type Boolean) (ElapsedSeconds :type Float%20%28double-precision%29) (TriggeredSeconds :type Float%20%28double-precision%29) (InputAction :type Input%20Action%20Object%20Reference :default "/Game/Game/Inputs/IA_Index_CC.IA_Index_CC"))
  ;[1 1 1] FINGERS
  (:Triggered
    (Variables|Default|SetIndex (* ElapsedSeconds 8e+01))
    (Variables|Default|SetRotatedIndex true))
  (:Completed
    (Variables|Default|SetRotatedIndex false)))

(event Input|EnhancedActionEvents|EnhancedInputActionIA_Extend
  (params (ActionValue :type Boolean) (ElapsedSeconds :type Float%20%28double-precision%29) (TriggeredSeconds :type Float%20%28double-precision%29) (InputAction :type Input%20Action%20Object%20Reference :default "/Game/Game/Inputs/IA_Extend.IA_Extend"))
  ;[1 1 1] ARM
  (:Started
    (Variables|Default|SetExtend true)
    (CallFunction|FREEZE))
  (:Completed
    (Variables|Default|SetExtend false)
    (CallFunction|UNFREEZE)))

(event Input|EnhancedActionEvents|EnhancedInputActionIA_Middle_CC
  (params (ActionValue :type Boolean) (ElapsedSeconds :type Float%20%28double-precision%29) (TriggeredSeconds :type Float%20%28double-precision%29) (InputAction :type Input%20Action%20Object%20Reference :default "/Game/Game/Inputs/IA_Middle_CC.IA_Middle_CC"))
  ;[1 1 1] FINGERS
  (:Triggered
    (Variables|Default|SetMiddle (* ElapsedSeconds 8e+01))
    (Variables|Default|SetRotatedMiddle true))
  (:Completed
    (Variables|Default|SetRotatedMiddle false)))

(event Input|EnhancedActionEvents|EnhancedInputActionIA_Thumb_CC
  (params (ActionValue :type Boolean) (ElapsedSeconds :type Float%20%28double-precision%29) (TriggeredSeconds :type Float%20%28double-precision%29) (InputAction :type Input%20Action%20Object%20Reference :default "/Game/Game/Inputs/IA_Thumb_CC.IA_Thumb_CC"))
  (bind _thumb_collision2 (Variables|Default|GetThumb_Collision2))
  (bind _camera (Variables|Default|GetCamera))
  (bind _returnvalue (Transformation|GetWorldLocation _thumb_collision2))
  (bind _returnvalue_2 (Transformation|GetWorldTransform _camera))
  ;[1 1 1] FINGERS
  (:Triggered
    (Variables|Default|SetThumb (* ElapsedSeconds 8e+01))
    (Variables|Default|SetRotatedThumb true)
    ;[1 1 1] Comment
    (if (Math|Boolean|ORBoolean (and (Variables|Default|GetIndexOverlapped) (Variables|Default|GetRotatedIndex)) (and (Variables|Default|GetRotatedMiddle) (Variables|Default|GetMiddle%20Overlapped)) (Variables|Default|GetRotatedOtherFingers))
      (bind (_outhit _returnvalue_3) (Collision|SphereTraceByChannel _returnvalue (+ _returnvalue (* (Math|Vector|GetForwardVector (Transformation|GetWorldRotation (Variables|Default|GetCamera))) 15.0)) 4.0 "TraceTypeQuery1" false 0 "ForDuration"))
      (if _returnvalue_3
        (bind _output_get (Variables|Default|SetImpact%20Point (.ImpactPoint (Collision|BreakHitResult _outhit))))
        (bind _output_get_2 (Variables|Default|SetHit%20Component (.HitComponent (Collision|BreakHitResult _outhit))))
        (Physics|Components|PhysicsHandle|GrabComponentatLocationwithRotation (Variables|Default|GetPhysicsHandle) _output_get_2 "None" _output_get (Math|Transform|InverseTransformRotation _returnvalue_2 (Transformation|GetWorldRotation _camera)))
        (Variables|Default|SetCanHoldCube true)
        (Variables|Default|SetImpact%20Point (Math|Transform|InverseTransformLocation _returnvalue_2 (Variables|Default|GetImpact%20Point)))
        (CallFunction|UpdateLoc))))
  (:Completed
    (Variables|Default|SetRotatedThumb false)
    (if (Variables|Default|GetCanHoldCube)
      (Physics|Components|PhysicsHandle|ReleaseComponent (Variables|Default|GetPhysicsHandle))
      (Variables|Default|SetCanHoldCube false))))

(event Input|EnhancedActionEvents|EnhancedInputActionIA_OtherFingers_CC
  (params (ActionValue :type Boolean) (ElapsedSeconds :type Float%20%28double-precision%29) (TriggeredSeconds :type Float%20%28double-precision%29) (InputAction :type Input%20Action%20Object%20Reference :default "/Game/Game/Inputs/IA_OtherFingers_CC.IA_OtherFingers_CC"))
  ;[1 1 1] FINGERS
  (:Triggered
    (Variables|Default|SetOtherFingers (* ElapsedSeconds 8e+01))
    (Variables|Default|SetRotatedOtherFingers true))
  (:Completed
    (Variables|Default|SetRotatedOtherFingers false)))

(event Input|EnhancedActionEvents|EnhancedInputActionIA_UpDownArm
  (params (ActionValue :type Boolean) (ElapsedSeconds :type Float%20%28double-precision%29) (TriggeredSeconds :type Float%20%28double-precision%29) (InputAction :type Input%20Action%20Object%20Reference :default "/Game/Game/Inputs/IA_UpDownArm.IA_UpDownArm"))
  ;[1 1 1] ARM
  (:Started
    (Variables|Default|SetArmUPDOWN true)
    (CallFunction|FREEZE))
  (:Completed
    (Variables|Default|SetArmUPDOWN false)
    (CallFunction|UNFREEZE)))

(event EventBeginPlay
  (bind _bone (Variables|Default|GetBone))
  ;[1 1 1] Ragdoll Hand
  (Class|PhysicalAnimationComponent|SetSkeletalMeshComponent (Variables|Default|GetPhysicalAnimation) (Variables|Default|GetGeneralSamHand))
  (Class|PhysicalAnimationComponent|ApplyPhysicalAnimationSettingsBelow (Variables|Default|GetPhysicalAnimation) _bone (Utilities|Struct|MakePhysicalAnimationData true 1e+03 1e+02 1e+03 1e+02 1e+02 1e+02) true)
  (Class|SkeletalMeshComponent|SetAllBodiesBelowSimulatePhysics (Variables|Default|GetGeneralSamHand) _bone true false))

(event EventPossessed
  (params (NewController :type Controller%20Object%20Reference))
  ;[1 1 1] MOVEMENT
  (bind _asplayer_controller (Utilities|Casting|CastToPlayerController NewController))
  (Input|AddMappingContext (PlayerController|LocalPlayerSubsystems|GetEnhancedInputLocalPlayerSubsystem _asplayer_controller) "/Game/Game/Inputs/Player_MappingContext.Player_MappingContext" 0 "(bIgnoreAllPressedKeysUntilRelease=True,bForceImmediately=False)"))

(fn ConstructionScript)

(fn FREEZE
  (Variables|/Script/Engine.CharacterMovementComponent|SetMaxWalkSpeed (Variables|Character|GetCharacterMovement) 5e+01)
  (Input|SetIgnoreLookInput (Game|GetPlayerController 0) true)
  (return))

(fn UNFREEZE
  (Variables|/Script/Engine.CharacterMovementComponent|SetMaxWalkSpeed (Variables|Character|GetCharacterMovement) (Variables|Default|GetWalkSpeed))
  (Input|ResetIgnoreLookInput (Game|GetPlayerController 0))
  (return))