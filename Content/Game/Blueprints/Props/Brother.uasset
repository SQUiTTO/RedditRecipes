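; Brother is a grabbable physics prop that reacts with a sound when a Cheesetest actor overlaps it.
; Tick attaches it to the player's hand socket when held and hit, or detaches it and restores physics when CanHoldCube is false.
; BeginPlay disables Tick, and the hand-scan logic that would re-enable it is disconnected.
; The cheese overlap sets Eat, destroys GrabCollision and plays a 2D sound from an array.
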(event OnComponentBeginOverlap(GrabCollision)
  (params (OverlappedComponent :type Primitive%20Component%20Object%20Reference) (OtherActor :type Actor%20Object%20Reference) (OtherComp :type Primitive%20Component%20Object%20Reference) (OtherBodyIndex :type Integer) (bFromSweep :type Boolean) (SweepResult :type Hit%20Result%20Structure%20%28by%20ref%29))
  (Utilities|Casting|CastToCheesetest OtherActor)
  (bind _output_get (Variables|Default|Seteat true))
  (if _output_get
    (Components|DestroyComponent (Variables|Default|GetGrabCollision))
    (Audio|PlaySound2D (Utilities|Array|Get(acopy) (Variables|Default|GetNewVar_0) (Variables|Default|GetNewVar)) 1.0 1.0 0.0 0 0)))

(event OnComponentEndOverlap(GrabCollision)
  (params (OverlappedComponent :type Primitive%20Component%20Object%20Reference) (OtherActor :type Actor%20Object%20Reference) (OtherComp :type Primitive%20Component%20Object%20Reference) (OtherBodyIndex :type Integer)))

(event EventBeginPlay
  (bind _asnew_player_bp (Utilities|Casting|CastToNewPlayer_BP (Game|GetPlayerCharacter 0)))
  (Variables|Default|SetAs%20New%20Player%20BP _asnew_player_bp)
  (Actor|Tick|SetActorTickEnabled self))

(event EventTick
  (params (DeltaSeconds :type Float%20%28single-precision%29))
  (bind _self self)
  (bind _as_new_player_bp (Variables|Default|GetAs%20New%20Player%20BP))
  (bind _hit_component (Variables|/Game/Game/Blueprints/Player/NewPlayer_BP.NewPlayer_BP_C|GetHit%20Component _as_new_player_bp))
  (bind _cube (Variables|Default|GetCube _self))
  (bind _returnvalue (Components|GetOwner _hit_component))
  (Variables|Default|SetCan%20Hold%20Cube (Variables|/Game/Game/Blueprints/Player/NewPlayer_BP.NewPlayer_BP_C|GetCanHoldCube (Variables|Default|GetAs%20New%20Player%20BP)))
  (if (Variables|Default|GetCan%20Hold%20Cube)
    (if (== _returnvalue self)
      (Transformation|AttachComponentToComponent (Variables|/Script/Engine.Actor|GetRootComponent _returnvalue) (Variables|/Game/Game/Blueprints/Player/NewPlayer_BP.NewPlayer_BP_C|GetGeneralSamHand _as_new_player_bp) "hand_rSocket" "KeepWorld" "KeepWorld" "KeepWorld" true)
      (Physics|SetSimulatePhysics _cube false)
      (Collision|SetCollisionEnabled _cube "PhysicsOnly"))
    (else
      (Transformation|DetachFromComponent (Variables|Transformation|GetRootComponent self) "KeepWorld" "KeepWorld" "KeepWorld" false)
      (Physics|SetSimulatePhysics (Variables|Default|GetCube) true)
      (Collision|SetCollisionEnabled (Variables|Default|GetCube) "QueryAndPhysics"))))

(fn ConstructionScript)