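; Physics cube prop that the player can pick up with the right hand and drop.
; Tick runs only while the player's HandScan overlaps GrabCollision, polling CanHoldCube and attaching the hit prop to the hand socket if the hand is empty.
; Physics is off while held; releasing CanHoldCube or ending the overlap detaches it and restores physics.
; A disconnected camera-trace procedural mesh slicing chain never runs.
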(event OnComponentBeginOverlap(GrabCollision)
  (params (OverlappedComponent :type Primitive%20Component%20Object%20Reference) (OtherActor :type Actor%20Object%20Reference) (OtherComp :type Primitive%20Component%20Object%20Reference) (OtherBodyIndex :type Integer) (bFromSweep :type Boolean) (SweepResult :type Hit%20Result%20Structure%20%28by%20ref%29))
  (if (== OtherComp (Variables|/Game/Game/Blueprints/Player/NewPlayer_BP.NewPlayer_BP_C|GetHandScan (Variables|Default|GetAs%20New%20Player%20BP)))
    (Actor|Tick|SetActorTickEnabled self true)))

(event OnComponentEndOverlap(GrabCollision)
  (params (OverlappedComponent :type Primitive%20Component%20Object%20Reference) (OtherActor :type Actor%20Object%20Reference) (OtherComp :type Primitive%20Component%20Object%20Reference) (OtherBodyIndex :type Integer))
  (if (== OtherComp (Variables|/Game/Game/Blueprints/Player/NewPlayer_BP.NewPlayer_BP_C|GetHandScan (Variables|Default|GetAs%20New%20Player%20BP)))
    (Actor|Tick|SetActorTickEnabled self)
    (Transformation|DetachFromComponent (Variables|Transformation|GetRootComponent self) "KeepWorld" "KeepWorld" "KeepWorld" false)
    (Variables|/Game/Game/Blueprints/Player/NewPlayer_BP.NewPlayer_BP_C|SetITEMinhand (Variables|Default|GetAs%20New%20Player%20BP) false)
    (Physics|SetSimulatePhysics (Variables|Default|GetCube) true)
    (Collision|SetCollisionEnabled (Variables|Default|GetCube) "QueryAndPhysics")))

(event EventBeginPlay
  (bind _asnew_player_bp (Utilities|Casting|CastToNewPlayer_BP (Game|GetPlayerCharacter 0)))
  (Variables|Default|SetAs%20New%20Player%20BP _asnew_player_bp)
  (Actor|Tick|SetActorTickEnabled self))

(event EventTick
  (params (DeltaSeconds :type Float%20%28single-precision%29))
  (bind _self self)
  (bind _as_new_player_bp (Variables|Default|GetAs%20New%20Player%20BP))
  (bind _as_new_player_bp_2 (Variables|Default|GetAs%20New%20Player%20BP))
  (bind _as_new_player_bp_3 (Variables|Default|GetAs%20New%20Player%20BP))
  (bind _hit_component (Variables|/Game/Game/Blueprints/Player/NewPlayer_BP.NewPlayer_BP_C|GetHit%20Component _as_new_player_bp_3))
  (bind _cube (Variables|Default|GetCube _self))
  (bind _returnvalue (Components|GetOwner _hit_component))
  (Variables|Default|SetCan%20Hold%20Cube (Variables|/Game/Game/Blueprints/Player/NewPlayer_BP.NewPlayer_BP_C|GetCanHoldCube _as_new_player_bp))
  (if (Variables|Default|GetCan%20Hold%20Cube)
    (if (not (Variables|/Game/Game/Blueprints/Player/NewPlayer_BP.NewPlayer_BP_C|GetITEMinhand _as_new_player_bp))
      (if (== _returnvalue self)
        (bind _returnvalue_2 (Transformation|AttachComponentToComponent (Variables|/Script/Engine.Actor|GetRootComponent _returnvalue) (Variables|/Game/Game/Blueprints/Player/NewPlayer_BP.NewPlayer_BP_C|GetGeneralSamHand _as_new_player_bp_3) "hand_rSocket" "KeepWorld" "KeepWorld" "KeepWorld" true))
        (Variables|/Game/Game/Blueprints/Player/NewPlayer_BP.NewPlayer_BP_C|SetITEMinhand _as_new_player_bp_2 _returnvalue_2)
        (Physics|SetSimulatePhysics _cube false)
        (Collision|SetCollisionEnabled _cube "PhysicsOnly")))
    (else
      (Transformation|DetachFromComponent (Variables|Transformation|GetRootComponent self) "KeepWorld" "KeepWorld" "KeepWorld" false)
      (Variables|/Game/Game/Blueprints/Player/NewPlayer_BP.NewPlayer_BP_C|SetITEMinhand _as_new_player_bp_2 false)
      (Physics|SetSimulatePhysics (Variables|Default|GetCube) true)
      (Collision|SetCollisionEnabled (Variables|Default|GetCube) "QueryAndPhysics"))))

(fn ConstructionScript)