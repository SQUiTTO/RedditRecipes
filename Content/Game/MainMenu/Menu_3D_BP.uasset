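; Menu_3D_BP is an actor for one screen of a 3D main menu, presenting a Menu_3D_Widget through a widget component.
; It starts with collision off and binds to the widget's transition event, whose index selects a target from its LinkedMenus array.
; A transition moves collision from this menu to the target and blends the player's view to that actor with an ease-in-out camera move.
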(event Custom|TransitionTo
  (params (New%20Menu :type Menu%203D%20BP%20Object%20Reference))
  (Collision|SetActorEnableCollision false)
  (Collision|SetActorEnableCollision New%20Menu true)
  (Game|Player|SetViewTargetwithBlend (Game|GetPlayerController 0) New%20Menu 2.0 "VTBlend_EaseInOut" 2.0 false))

(event Custom|OnTransitionBetweenMenus
  (params (MenuIndex :type Integer))
  (if (Utilities|Array|IsValidIndex (Variables|Default|GetLinkedMenus) MenuIndex)
    (CallFunction|Transitionto (Utilities|Array|Get(acopy) (Variables|Default|GetLinkedMenus) MenuIndex))))

(event EventBeginPlay
  (bind _asmenu_3d_widget (Utilities|Casting|CastToMenu_3D_Widget (UserInterface|GetUserWidgetObject (Variables|Default|GetWidget))))
  (EventDispatchers|AssignTransitiontoLinkedMenu _asmenu_3d_widget (delegate Custom|OnTransitionBetweenMenus))
  (Collision|SetActorEnableCollision false))

(fn ConstructionScript)